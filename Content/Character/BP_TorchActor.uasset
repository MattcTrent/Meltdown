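; The player's torch, a spotlight with a power percentage that sets its intensity and ends the game when drained.
; A looping timer started on game start drains power, while AddPower restores it up to full.
; Damage drains briefly show an electrical particle effect and fire notifications.
; Box and sphere overlaps toggle outlines on BP_Key actors the light touches.
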(event OnComponentBeginOverlap(Box)
  (params (OverlappedComponent :type Primitive%20Component%20Object%20Reference) (OtherActor :type Actor%20Object%20Reference) (OtherComp :type Primitive%20Component%20Object%20Reference) (OtherBodyIndex :type Integer) (bFromSweep :type Boolean) (SweepResult :type Hit%20Result%20Structure%20%28by%20ref%29))
  ;[1 1 1] overlay when light hits
  (bind _asbp_key (Utilities|Casting|CastToBP_Key OtherActor))
  (Default|OutlineforObject _asbp_key self true)
  (Variables|Default|Setstill%20in%20coll? true))

(event OnComponentBeginOverlap(Sphere)
  (params (OverlappedComponent :type Primitive%20Component%20Object%20Reference) (OtherActor :type Actor%20Object%20Reference) (OtherComp :type Primitive%20Component%20Object%20Reference) (OtherBodyIndex :type Integer) (bFromSweep :type Boolean) (SweepResult :type Hit%20Result%20Structure%20%28by%20ref%29))
  ;[1 1 1] overlay when light hits
  (bind _asbp_key (Utilities|Casting|CastToBP_Key OtherActor))
  (Default|OutlineforObject _asbp_key self true)
  (Variables|Default|Setstill%20in%20box%20coll? true))

(event OnComponentEndOverlap(Sphere)
  (params (OverlappedComponent :type Primitive%20Component%20Object%20Reference) (OtherActor :type Actor%20Object%20Reference) (OtherComp :type Primitive%20Component%20Object%20Reference) (OtherBodyIndex :type Integer))
  ;[1 1 1] end outline when not hitting
  (bind _asbp_key (Utilities|Casting|CastToBP_Key OtherActor))
  (Default|OutlineforObject _asbp_key self false)
  (Variables|Default|Setstill%20in%20coll? false))

(event OnComponentEndOverlap(Box)
  (params (OverlappedComponent :type Primitive%20Component%20Object%20Reference) (OtherActor :type Actor%20Object%20Reference) (OtherComp :type Primitive%20Component%20Object%20Reference) (OtherBodyIndex :type Integer))
  ;[1 1 1] end outline when not hitting
  (bind _asbp_key (Utilities|Casting|CastToBP_Key OtherActor))
  (Default|OutlineforObject _asbp_key self false)
  (Variables|Default|Setstill%20in%20box%20coll? false))

(event Custom|Start%20Torch%20Timer
  (bind _returnvalue (Utilities|Time|SetTimerbyFunctionName 0 "PowerDrain" (Variables|Default|GetDrainTime) true))
  (Variables|Default|SetTimerHandle _returnvalue))

(event Custom|ResetNotify
  (Utilities|FlowControl|DoOnce false) ; enters at Reset
)

(event Custom|Init%20Torch
  (bind _self self)
  (bind _persistantgm (CallFunction|GetGameMode _self))
  (CallFunction|SetVariables)
  (EventDispatchers|BindEventtoOnStartGame _persistantgm (delegate Custom|Start%20Torch%20Timer))
  (EventDispatchers|BindEventtoMenuLoaded (Variables|/Game/GameModes/BP_PersistantGM.BP_PersistantGM_C|GetLevelStreamManager _persistantgm) (EventDispatchers|CreateEvent :!event Custom|ResetNotify))
  (Components|Activation|SetActive (Variables|Default|GetElectricalEffect) false true))

(event Custom|PauseDrainTimer
  (Utilities|Time|PauseTimerbyHandle (Variables|Default|GetTimerHandle)))

(event Custom|ResumeDrainTimer
  (Utilities|Time|UnpauseTimerbyHandle (Variables|Default|GetTimerHandle)))

(event Custom|CallEndGameNotify
  (Utilities|FlowControl|DoOnce false
    (:Completed
      (Default|CallOnEndGame (CallFunction|GetGameMode self))
      (Utilities|Time|ClearandInvalidateTimerbyHandle (Variables|Default|GetTimerHandle))
      (Variables|Default|SetPowerPercent (Variables|Default|GetTorchStartAmount)))))

(event Custom|ResetCharge
  (Variables|Default|SetPowerPercent 100))

(fn ConstructionScript)

(fn PowerDrain
  (CallFunction|ReducePower (Variables|Default|GetDrainTick) "0, 0, 0" false))

(fn ReducePower
  (params (PercentToReduce :type Integer) (location :type Vector) (Is%20being%20damaged? :type Boolean))
  (bind _electricaleffect (Variables|Default|GetElectricalEffect))
  (if (<= (- (Variables|Default|GetPowerPercent) PercentToReduce) 0)
    (bind _output_get (Variables|Default|SetPowerPercent 0))
    (bind _output_get_2 (Variables|Default|SetCurrentIntensity (* _output_get (Variables|Default|GetIntensityPerPercent))))
    (Rendering|Components|Light|SetIntensity (Variables|Default|GetSpotLight) _output_get_2)
    (CallFunction|CallEndGameNotify)
    (else
      (bind _output_get_3 (Variables|Default|SetPowerPercent (- (Variables|Default|GetPowerPercent) PercentToReduce)))
      (bind _output_get_4 (Variables|Default|SetCurrentIntensity (* _output_get_3 (Variables|Default|GetIntensityPerPercent))))
      (Rendering|Components|Light|SetIntensity (Variables|Default|GetSpotLight) _output_get_4)
      (if Is%20being%20damaged?
        ;[1 1 1] matt d add
        (if (not (Variables|Default|Getis%20damaging))
          (Development|SetHiddeninGame _electricaleffect false false)
          (Components|Activation|SetActive _electricaleffect true false)
          (Variables|Default|Setis%20damaging true)
          (Utilities|Time|SetTimerbyFunctionName 0 "TurnParticle effect off" 2.8)
          (Default|CallOnParticleon))))))

(fn AddPower
  (params (PercentToAdd :type Integer))
  (if (>= (+ PercentToAdd (Variables|Default|GetPowerPercent)) 100)
    (bind _output_get (Variables|Default|SetPowerPercent 100))
    (bind _output_get_2 (Variables|Default|SetCurrentIntensity (* _output_get (Variables|Default|GetIntensityPerPercent))))
    (Rendering|Components|Light|SetIntensity (Variables|Default|GetSpotLight) _output_get_2)
    (else
      (bind _output_get_3 (Variables|Default|SetPowerPercent (+ PercentToAdd (Variables|Default|GetPowerPercent))))
      (bind _output_get_4 (Variables|Default|SetCurrentIntensity (* _output_get_3 (Variables|Default|GetIntensityPerPercent))))
      (Rendering|Components|Light|SetIntensity (Variables|Default|GetSpotLight) _output_get_4)
      (Default|CallOnEnergyGained))))

(fn SetVariables
  (bind _maxintensity (Variables|Default|GetMaxIntensity))
  (Rendering|Components|Light|SetIntensity (Variables|Default|GetSpotLight) _maxintensity)
  (Variables|Default|SetCurrentIntensity _maxintensity)
  (Variables|Default|SetIntensityPerPercent (* _maxintensity 0.01))
  (Variables|Default|SetPowerPercent 100))

(fn TurnParticleEffectOff
  (bind _electricaleffect (Variables|Default|GetElectricalEffect))
  (Components|Activation|SetActive _electricaleffect false true)
  (Variables|Default|Setis%20damaging false)
  (Development|SetHiddeninGame _electricaleffect true false)
  (Default|CallOnParticleOff))