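; Player character Blueprint that sets up the camera look, a torch and on-screen tutorials.
; Init copies settings from the "World"-tagged BP_PostProcess to the camera, initialises the child-actor torch and shows timed intro tutorials.
; InteractCollision overlaps with keys, interactable doors and NPCs show contextual hints on the tutorial widget component, gated by first-interaction flags.
; MiniMapInit registers the character with the game mode, and IconType exposes its icon type.
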(event OnComponentBeginOverlap(InteractCollision)
  (params (OverlappedComponent :type Primitive%20Component%20Object%20Reference) (OtherActor :type Actor%20Object%20Reference) (OtherComp :type Primitive%20Component%20Object%20Reference) (OtherBodyIndex :type Integer) (bFromSweep :type Boolean) (SweepResult :type Hit%20Result%20Structure%20%28by%20ref%29))
  ;[1 1 1] Interaction Tutorials
  ;;[1 1 1] If overlapping Key and Not interacted with a Key, Show Key Tutorial
  (Utilities|Casting|CastToBP_Key OtherActor
    (:then
      (if (not (Variables|Default|GetFirstKey))
        (Default|SetText (CallFunction|GetTutorialUI) "NewEnumerator3")))
    (:CastFailed
      ;;[1 1 1] If overlapping Door and Not interacted with a Door, Show Door Tutorial
      (Utilities|Casting|CastToBP_Door_Interactable OtherActor
        (:then
          (if (not (Variables|Default|GetFirstDoor))
            (Default|SetText (CallFunction|GetTutorialUI) "NewEnumerator4")))
        (:CastFailed
          ;;[1 1 1] If overlapping NPC and Not interacted with a NPC, Show NPC Tutorial
          (Utilities|Casting|CastToBP_NPCChar OtherActor)
          (if (not (Variables|Default|GetFirstNPC))
            (Default|SetText (CallFunction|GetTutorialUI) "NewEnumerator5")))))))

(event Custom|Get%20Post%20Process
  ;[1 1 1] Setup Post Process
  (bind _outactors (Actor|GetAllActorsOfClass "/Game/GameplayObjects/BP_PostProcess.BP_PostProcess_C"))
  (bind _array_element (Utilities|Array|ForEachLoopwithBreak _outactors :!label _label)
    (:LoopBody
      (if (Components|ComponentHasTag (Variables|/Game/GameplayObjects/BP_PostProcess.BP_PostProcess_C|GetPostProcess _array_element) "World")
        (Variables|Default|SetPost%20Process _array_element)
        (goto _label Break)))
    (:Completed
      (CallFunction|SetPostProcessSetting))))

(event Custom|Init
  ;[1 1 1] Initialisation Sequence
  (CallFunction|GetPostProcess)
  (CallFunction|InitPlayerTorch)
  (CallFunction|DisplayTutorials))

(event Custom|MiniMapInit
  (bind _self self)
  ;[1 1 1] Initialise Minimap
  (Default|CallOnObjectInitialised (CallFunction|GetGameMode _self) _self))

(event Custom|Display%20Tutorials
  (bind _widget (Variables|Default|GetWidget))
  (bind _returnvalue (UserInterface|GetUserWidgetObject _widget))
  (bind _aswbp_tutorial (Utilities|Casting|CastToWBP_Tutorial _returnvalue))
  ;[1 1 1] Tutorial Calls
  (Utilities|FlowControl|Delay 1.0)
  (Development|SetHiddeninGame _widget false true)
  (Default|SetText _aswbp_tutorial "NewEnumerator0")
  (Utilities|FlowControl|Delay 3.5)
  (Default|SetText _aswbp_tutorial "NewEnumerator2"))

(event EventTick
  (params (DeltaSeconds :type Float%20%28single-precision%29))
  ;[1 1 1] Tick
  (|CallParentFunction DeltaSeconds))

(fn ConstructionScript
  (|CallParentFunction))

(fn SetPostProcessSetting
  (Variables|/Script/Engine.CameraComponent|SetPostProcessSettings (Variables|Default|GetCamera) (Variables|/Script/Engine.PostProcessComponent|GetSettings (Variables|/Game/GameplayObjects/BP_PostProcess.BP_PostProcess_C|GetPostProcess (Variables|Default|GetPost%20Process)))))

(fn InitPlayerTorch
  (Default|InitTorch (.AsBP%20Torch%20Actor (Utilities|Casting|CastToBP_TorchActor (Variables|/Script/Engine.ChildActorComponent|GetChildActor (Variables|Default|GetTorchActor))))))

(fn GetTutorialUI
  (return (.AsWBP%20Tutorial (Utilities|Casting|CastToWBP_Tutorial (UserInterface|GetUserWidgetObject (Variables|Default|GetWidget))))))

(fn IconType
  (return (Variables|Default|GetIcon%20Type)))