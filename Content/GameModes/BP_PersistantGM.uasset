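; Persistent-level GameMode that runs the game flow from menu through game over, tracking player controllers in the GameInstance on login and logout.
; BeginPlay initializes the level stream manager, binds phase events, streams in the menu level and fires pre-start.
; Pre-start sets up spawn and narrative managers and spawns players; start records positions; end shows game-over UI.
; Respawn functions teleport Player1 to main-menu or level-one checkpoints.
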(event Custom|SetupBindings
  ;[1 1 1] setup refrences and bindings
  (Utilities|FlowControl|Sequence
    (:then_0
      (EventDispatchers|BindEventtoOnPreStart (delegate Custom|OnPreStart_Event)))
    (:then_1
      (EventDispatchers|BindEventtoOnStartGame (delegate Custom|OnStartGame_Event)))
    (:then_2
      (EventDispatchers|BindEventtoOnEndGame (delegate Custom|OnEndGame_Event)))))

(event Custom|OnPreStart_Event
  ;[1 1 1] setup refrences and bindings
  (CallFunction|InitSpawnManagers) ; WILL NEED TO DISCUSS THIS AS SOME MANAGERS WILL ONLY NEED TO EXIST IN LEVEL ONE LIKE THE NARRATIVE MANAGER AS IT NEEDS TO GET REFS TO NPC'S
  (CallFunction|SpawnAllPlayers))

(event Custom|Retry%20game)

(event Custom|back%20to%20menu)

(event Custom|OnEndGame_Event
  ;[1 1 1] setup refrences and bindings
  (CallFunction|EndGameCondition))

(event Custom|Load%20Menu
  (Game|LoadStreamLevel(byName) "Level_Menu" true))

(event Custom|Level%20One%20Started
  (Development|PrintString "COUNT DOWN STARTED" true true "(R=0.000000,G=1.000000,B=0.000306,A=1.000000)")
  (for _array_element (Variables|/Game/BP_GameInstance.BP_GameInstance_C|GetPlayers (CallFunction|GetGameInstance self))
    (Utilities|Array|Add (Variables|Default|GetPlayer%20level%20one%20start%20positions) (Transformation|GetActorLocation (Pawn|GetControlledPawn _array_element)))))

(event Custom|Quit%20Game
  ;[0.1414 0 1] ADDED TO GM
  (Game|QuitGame (Game|GetPlayerController 0) "Quit"))

(event Custom|OnStartGame_Event
  ;[1 1 1] setup refrences and bindings
  (CallFunction|LevelOneStarted))

(event Custom|Get%20Stream%20Manager
  (bind _outactors (Actor|GetAllActorsOfClass "/Game/Managers/BP_LevelStreamManager.BP_LevelStreamManager_C"))
  (bind _output_get (Variables|Default|SetLevelStreamManager (Utilities|Array|Get(acopy) _outactors)))
  (Default|InitLevelStreamManager _output_get self))

(event EventBeginPlay
  (CallFunction|GetStreamManager)
  (CallFunction|SetupBindings)
  (CallFunction|LoadMenu)
  (Default|CallOnPreStart))

(event EventPostLogin
  (params (NewPlayer :type Player%20Controller%20Object%20Reference))
  (bind _self self)
  (bind _game_instance (CallFunction|GetGameInstance _self))
  (bind _players (Variables|/Game/BP_GameInstance.BP_GameInstance_C|GetPlayers _game_instance))
  ;[1 1 1] Handle Log in/out
  (bind _asbp_player_controller (Utilities|Casting|CastToBP_PlayerController NewPlayer)
    (:then
      (Utilities|Array|AddUnique _players _asbp_player_controller)
      (if (== (Utilities|Array|Length _players) 1)
        (Variables|Default|Setplayer%201 _asbp_player_controller)))
    (:CastFailed
      (Development|PrintString "player controller cast failted in maingm" true true "(R=1.000000,G=0.000000,B=0.120615,A=1.000000)" 9e+01))))

(event EventOnLogout
  (params (ExitingController :type Controller%20Object%20Reference))
  ;[1 1 1] Handle Log in/out
  (bind _asbp_player_controller (Utilities|Casting|CastToBP_PlayerController ExitingController))
  (Utilities|Array|RemoveItem (Variables|/Game/BP_GameInstance.BP_GameInstance_C|GetPlayers (CallFunction|GetGameInstance self)) _asbp_player_controller))

(fn ConstructionScript)

(fn InitSpawnManagers
  (for _array_element (Variables|/Game/BP_GameInstance.BP_GameInstance_C|GetPlayers (CallFunction|GetGameInstance self))
    (Default|InitSM _array_element))
  (CallFunction|InitNarrativeManager))

(fn SpawnAllPlayers
  (for _array_element (Variables|/Game/BP_GameInstance.BP_GameInstance_C|GetPlayers (CallFunction|GetGameInstance self))
    (Default|CallOnSpawnCharacter _array_element _array_element)
    (Utilities|Array|Add (Variables|Default|GetPlayer%20start%20positions) (Transformation|GetActorLocation (Pawn|GetControlledPawn _array_element)))))

(fn InitNarrativeManager
  ;[1 1 1] matt d's narrative manager
  (bind _returnvalue (Game|SpawnActorfromClass "/Game/Managers/BP_NarrativeManager.BP_NarrativeManager_C" (Math|Transform|MakeTransform "0, 0,2000.000000" "0, 0, 0" "1,1,1") "Undefined" 0 0))
  (bind _output_get (Variables|Default|Setnarrative%20manager%20ref _returnvalue))
  (Default|InitNarrtiveManager _output_get (Utilities|Array|Get(acopy) (Variables|/Game/BP_GameInstance.BP_GameInstance_C|GetPlayers (CallFunction|GetGameInstance self)))))

(fn GetMenuCam
  (bind _outactors (Actor|GetAllActorsOfClass "/Script/Engine.CameraActor"))
  (bind _array_element (Utilities|Array|ForEachLoopwithBreak _outactors)
    (:LoopBody
      (if (Components|ComponentHasTag (Variables|/Script/Engine.CameraActor|GetCameraComponent _array_element) "MenuCam")
        (LocalVariables|SetTemp%20Cam _array_element)))
    (:Completed
      (return (LocalVariables|GetTemp%20Cam)))))

(fn StartGme)

(fn EndGameCondition
  (Development|PrintString "game over" true true "(R=1.000000,G=0.000000,B=0.069748,A=1.000000)" 9e+01)
  (bind _returnvalue (UserInterface|CreateWidget "/Game/UI/WBP_GameOverUI.WBP_GameOverUI_C" (Game|GetPlayerController 0)))
  (bind _output_get (Variables|Default|SetGameOver%20UI _returnvalue))
  (UserInterface|Viewport|AddtoViewport _output_get 0)
  (Default|INIT _output_get self))

(fn RespawningtoStartOfLevel1
  (bind _player_1 (Variables|Default|Getplayer%201))
  (bind _controlledchar (Variables|/Game/PlayerControllers/BP_PlayerController.BP_PlayerController_C|GetControlledChar _player_1))
  (bind _array_element (Utilities|Array|ForEachLoopwithBreak (Variables|/Game/Managers/BP_SpawnManager.BP_SpawnManager_C|GetCheckpoints (Variables|/Game/PlayerControllers/BP_PlayerController.BP_PlayerController_C|GetBP_SpawnManager _player_1)))
    (:LoopBody
      (if (== (Variables|/Game/Managers/BP_PlayerCheckpoint.BP_PlayerCheckpoint_C|GetCheckpoint _array_element) 1)
        (bind _returnvalue (Transformation|Teleport _controlledchar (Transformation|GetActorLocation _array_element) (Transformation|GetActorRotation _controlledchar)))
        (if (not _returnvalue)
          (Development|PrintString "cant move me" true true "(R=1.000000,G=0.000000,B=0.358160,A=1.000000)" 9e+01))))))

(fn RespawningtoMainMenu
  (bind _player_1 (Variables|Default|Getplayer%201))
  (bind _controlledchar (Variables|/Game/PlayerControllers/BP_PlayerController.BP_PlayerController_C|GetControlledChar _player_1))
  (bind _array_element (Utilities|Array|ForEachLoopwithBreak (Variables|/Game/Managers/BP_SpawnManager.BP_SpawnManager_C|GetCheckpoints (Variables|/Game/PlayerControllers/BP_PlayerController.BP_PlayerController_C|GetBP_SpawnManager _player_1)))
    (:LoopBody
      (if (Variables|/Game/Managers/BP_PlayerCheckpoint.BP_PlayerCheckpoint_C|GetMainMenu? _array_element)
        (bind _returnvalue (Transformation|Teleport _controlledchar (Transformation|GetActorLocation _array_element) (Transformation|GetActorRotation _controlledchar)))
        (if (not _returnvalue)
          (Development|PrintString "cant move me" true true "(R=1.000000,G=0.000000,B=0.358160,A=1.000000)" 9e+01))))))