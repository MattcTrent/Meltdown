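; Narrative manager that sets up NPC dialogue widgets with random lines and names, with unfinished handling for player-to-NPC interaction.
; Init stores the GameMode and PlayerController, binds to the person-saved event and creates a dialog widget.
; NPC updates fill each NPC's widget, flagging ID 0 as first, then bind interaction events whose handlers are empty.
; Names, and lines for other NPCs, are removed at separately rolled random indices.
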(event Custom|init%20narrtive%20manager
  (params (player%20controller :type BP%20Player%20Controller%20Object%20Reference) (GM :type BP%20Persistant%20GM%20Object%20Reference))
  ;[0 0.05359 1] listening for when player speaks to npc
  (bind _output_get (Variables|Default|SetGM GM))
  (Variables|Default|Setplayer%20controller player%20controller)
  (EventDispatchers|BindEventtoPersonSaved _output_get (delegate Custom|player%20speaking%20to%20npc))
  (CallFunction|SETUPUi))

(event Custom|update%20npc%20when%20player%20moves
  (params (NPC's :type Array%20of%20BP%20NPC%20Char%20Object%20References))
  (Variables|Default|SetNPC's NPC's)
  (bind _npc_s (CallFunction|SetupNPC))
  (for _array_element _npc_s
    (EventDispatchers|BindEventtoOnInteractedwithPlayer _array_element (delegate Custom|npc))))

(event Custom|player%20speaking%20to%20npc
  (params (room :type BP%20Room%20Manager%20Object%20Reference))
  ;[0 0.05359 1] listening for when player speaks to npc
)

(event Custom|npc
  (params (Actor :type BP%20NPC%20Char%20Object%20Reference)))

(fn ConstructionScript)

(fn ManageNarrtiveDialogue
  (params (Selection :type NPC_names%20Enum :default "NewEnumerator0"))
  (switch Utilities|FlowControl|Switch|SwitchonNPC_names Selection))

(fn SETUPUi
  (bind _player_controller (Variables|Default|Getplayer%20controller))
  (Utilities|IsValid _player_controller
    (:Is%20Valid
      (bind _returnvalue (UserInterface|CreateWidget "/Game/UI/NPCDialogue/WBP_NarrativeDialog.WBP_NarrativeDialog_C" _player_controller))
      (Variables|Default|SetUI%20ref _returnvalue)
      ;[1 1 1] change in future once have ref in gamemode
      (bind _foundwidgets (Widget|GetAllWidgetsOfClass "/Game/UI/WBP_MasterGameHud.WBP_MasterGameHud_C" true)))
    (:Is%20Not%20Valid
      (Development|PrintString "narrative manager controller not valid!!!!!" true true "(R=1.000000,G=0.000000,B=0.022033,A=1.000000)" 9e+01))))

(fn SetupNPC
  (bind _returnvalue (Utilities|GetHowManyNames))
  (bind _npclines (Variables|Default|GetNPCLines))
  (bind _returnvalue_2 (Math|Random|RandomIntegerinRange 0 _returnvalue))
  ;[1 1 1] set text an names
  (for _array_element (Variables|Default|GetNPC's)
    (if (== (Variables|/Game/GameplayObjects/Interactables/BP_NPCChar.BP_NPCChar_C|GetNPC_ID _array_element) 0)
      ;[1 1 1] if its the first NPC in pool room
      (bind _aswbp_narrative_dialog (Utilities|Casting|CastToWBP_NarrativeDialog (UserInterface|GetUserWidgetObject (Variables|/Game/GameplayObjects/Interactables/BP_NPCChar.BP_NPCChar_C|GetWidget _array_element))))
      (Default|SetTextforNpc _aswbp_narrative_dialog (Utilities|Array|Get(acopy) (Variables|Default|GetNPCLines) (Math|Random|RandomIntegerinRange 0 (Utilities|GetHowManyNames))) _array_element true)
      (CallFunction|ChooseNpcName _aswbp_narrative_dialog)
      (else
        (bind _aswbp_narrative_dialog_2 (Utilities|Casting|CastToWBP_NarrativeDialog (UserInterface|GetUserWidgetObject (Variables|/Game/GameplayObjects/Interactables/BP_NPCChar.BP_NPCChar_C|GetWidget _array_element))))
        (Default|SetTextforNpc _aswbp_narrative_dialog_2 (Utilities|Array|Get(acopy) _npclines _returnvalue_2) _array_element false)
        (Utilities|Array|RemoveIndex _npclines _returnvalue_2)
        (CallFunction|ChooseNpcName _aswbp_narrative_dialog_2))))
  (return (Variables|Default|GetNPC's)))

(fn ChooseNpcName
  (params (self2 :type WBP%20Narrative%20Dialog%20Object%20Reference))
  (bind _returnvalue (Utilities|GetHowManyNames))
  (bind _names (Variables|Default|Getnames))
  (bind _returnvalue_2 (Math|Random|RandomIntegerinRange 0 _returnvalue))
  (Default|SetTextNPCName self2 (Utilities|Array|Get(acopy) _names _returnvalue_2))
  (Utilities|Array|RemoveIndex _names _returnvalue_2))