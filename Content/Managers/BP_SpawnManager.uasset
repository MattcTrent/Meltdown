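; BP_SpawnManager spawns a player's character at their team's checkpoint until the game ends.
; Initialise stores the DCPlayer, caches BP_PlayerCheckpoint actors matching its team and binds to the player's spawn and game mode's end-game events.
; Spawn requests use the checkpoint matching the player's current one, with unit scale.
; TempSpawn is never cleared, so the first cached checkpoint is the fallback only while it is invalid.
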(event Custom|Initialise
  (params (DCPlayer :type BP%20Player%20Controller%20Object%20Reference))
  (Variables|Default|SetDCPlayer DCPlayer)
  (CallFunction|GetAllCheckpoint)
  (EventDispatchers|AssignOnEndGame (CallFunction|GetGameMode self) (delegate Custom|OnEndGame_Event))
  (EventDispatchers|AssignOnSpawnCharacter (Variables|Default|GetDCPlayer) (delegate Custom|OnSpawnCharacter_Event))
  (Variables|Default|SetSpawn%20Enabled true))

(event Custom|OnSpawnCharacter_Event
  (params (PC :type BP%20Player%20Controller%20Object%20Reference))
  (if (Variables|Default|GetSpawn%20Enabled)
    (bind _spawnlocation (CallFunction|GetSpawnPoint))
    (Default|SpawnCharacter PC _spawnlocation)))

(event Custom|OnEndGame_Event
  (Variables|Default|SetSpawn%20Enabled false))

(fn GetAllCheckpoint
  (Utilities|Array|Clear (Variables|Default|GetCheckpoints))
  (bind _outactors (Actor|GetAllActorsOfClass "/Game/Managers/BP_PlayerCheckpoint.BP_PlayerCheckpoint_C"))
  (for _array_element _outactors
    (if (== (Variables|/Game/Managers/BP_PlayerCheckpoint.BP_PlayerCheckpoint_C|GetTeamNo _array_element) (Variables|/Game/PlayerControllers/BP_PlayerController.BP_PlayerController_C|GetTeamNo (Variables|Default|GetDCPlayer)))
      (Utilities|Array|Add (Variables|Default|GetCheckpoints) _array_element))))

(fn GetSpawnPoint
  (bind _checkpoints (Variables|Default|GetCheckpoints))
  (bind _output (Utilities|Array|Get(acopy) _checkpoints))
  (bind _returnvalue (Transformation|GetActorTransform _output))
  (bind (_location _rotation) (Math|Transform|BreakTransform _returnvalue))
  (for _array_element (Variables|Default|GetCheckpoints)
    (if (== (Variables|/Game/Managers/BP_PlayerCheckpoint.BP_PlayerCheckpoint_C|GetCheckpoint _array_element) (Variables|/Game/PlayerControllers/BP_PlayerController.BP_PlayerController_C|GetCheckpoint (Variables|Default|GetDCPlayer)))
      (LocalVariables|SetTempSpawn _array_element)))
  (Utilities|IsValid (LocalVariables|GetTempSpawn)
    (:Is%20Valid
      (return (Math|Transform|MakeTransform (.Location (Math|Transform|BreakTransform (Transformation|GetActorTransform (LocalVariables|GetTempSpawn)))) (.Rotation (Math|Transform|BreakTransform (Transformation|GetActorTransform (LocalVariables|GetTempSpawn)))))))
    (:Is%20Not%20Valid
      (return (Math|Transform|MakeTransform _location _rotation)))))