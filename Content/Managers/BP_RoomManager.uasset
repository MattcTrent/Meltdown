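; BP_RoomManager sets up a room when the player enters its Box trigger, restoring prior progress on keys, doors and NPCs.
; A DoOnce, re-armed by the Leave trigger, gates rebuilding actor arrays filtered by the room's ID ranges and binding keys to the HUD.
; It then replays picked-up, opened and rescued states from the player's key array and its own door/NPC arrays.
; Finally, it notifies the GM reference that the room initialised.
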(event OnComponentBeginOverlap(Box)
  (params (OverlappedComponent :type Primitive%20Component%20Object%20Reference) (OtherActor :type Actor%20Object%20Reference) (OtherComp :type Primitive%20Component%20Object%20Reference) (OtherBodyIndex :type Integer) (bFromSweep :type Boolean) (SweepResult :type Hit%20Result%20Structure%20%28by%20ref%29))
  (Utilities|FlowControl|DoOnce false
    (:Completed
      (bind _asbp_player_character (Utilities|Casting|CastToBP_PlayerCharacter OtherActor))
      ;[1 1 1] Clear All Arrays
      (Variables|Default|Setchar _asbp_player_character)
      (Utilities|Array|Clear (Variables|Default|GetKeyArray))
      (Utilities|Array|Clear (Variables|Default|GetDoorArray))
      (Utilities|Array|Clear (Variables|Default|GetNPCArray))
      (Utilities|FlowControl|Sequence
        (:then_0
          ;[1 1 1] Init All Arrays
          (CallFunction|DoorsInitialised))
        (:then_1
          (CallFunction|KeysInitialised))
        (:then_2
          (CallFunction|NPCsInitialised))
        (:then_3
          ;[1 1 1] Handle Key Picked Up
          (for _index (range (Variables|Default|GetMinKeyID) (Variables|Default|GetMaxKeyID))
            (if (Utilities|Array|Get(acopy) (Variables|/Game/Character/BP_PlayerCharacter.BP_PlayerCharacter_C|GetKeyArray (Variables|Default|Getchar)) _index)
              (for _array_element (Variables|Default|GetKeyArray)
                (if (== (Variables|/Game/GameplayObjects/Interactables/BP_Key.BP_Key_C|GetKeyNum _array_element) _index)
                  (Default|AlreadyPickedUp _array_element)))))
          ;[1 1 1] Handle Door Interacted
          (for (_array_element_2 _array_index) (Variables|Default|GetOpenDoors)
            (if _array_element_2
              (for _array_element_3 (Variables|Default|GetDoorArray)
                (if (== (Variables|/Game/GameplayObjects/Interactables/BP_Door_Interactable.BP_Door_Interactable_C|GetDoorID _array_element_3) _array_index)
                  (Default|OpenDoors _array_element_3)))))
          ;[1 1 1] Handle NPC Interaction
          (for (_array_element_4 _array_index_2) (Variables|Default|GetRescuedNPCs)
            (if _array_element_4
              (for _array_element_5 (Variables|Default|GetNPCArray)
                (if (== (Variables|/Game/GameplayObjects/Interactables/BP_NPCChar.BP_NPCChar_C|GetNPC_ID _array_element_5) _array_index_2)
                  (Default|AlreadySaved _array_element_5))))))
        (:then_4
          ;[1 1 1] moved here
          (Default|CallOnRoomInit (Variables|Default|GetGMref) self))))))

(event OnComponentBeginOverlap(Leave)
  (params (OverlappedComponent :type Primitive%20Component%20Object%20Reference) (OtherActor :type Actor%20Object%20Reference) (OtherComp :type Primitive%20Component%20Object%20Reference) (OtherBodyIndex :type Integer) (bFromSweep :type Boolean) (SweepResult :type Hit%20Result%20Structure%20%28by%20ref%29))
  (Utilities|FlowControl|DoOnce false) ; enters at Reset
)

(event Custom|init%20room
  (params (GM :type BP%20Persistant%20GM%20Object%20Reference))
  ;[1 1 1] Initialise GM Ref
  (Variables|Default|SetGMref GM))

(event Custom|ResetArrays
  (bind _opendoors (Variables|Default|GetOpenDoors))
  (bind _rescuednpcs (Variables|Default|GetRescuedNPCs))
  ;[1 1 1] Reset Arrays for Doors and NPC
  (for (_ _array_index) _opendoors
    (Utilities|Array|SetArrayElem _opendoors _array_index false))
  (for (_ _array_index_2) _rescuednpcs
    (Utilities|Array|SetArrayElem _rescuednpcs _array_index_2 false)))

(fn ConstructionScript)

(fn NPCsInitialised
  (bind _outactors (Actor|GetAllActorsOfClass "/Game/GameplayObjects/Interactables/BP_NPCChar.BP_NPCChar_C"))
  (for _array_element _outactors
    (Default|Init _array_element self)
    (if (Math|Integer|InRange(Integer) (Variables|/Game/GameplayObjects/Interactables/BP_NPCChar.BP_NPCChar_C|GetNPC_ID _array_element) (Variables|Default|GetMinNPC_ID) (Variables|Default|GetMaxNPC_ID))
      (Utilities|Array|Add (Variables|Default|GetNPCArray) _array_element))))

(fn KeysInitialised
  (bind _outactors (Actor|GetAllActorsOfClass "/Game/GameplayObjects/Interactables/BP_Key.BP_Key_C"))
  (for _array_element _outactors
    (Default|Init _array_element)
    (if (Math|Integer|InRange(Integer) (Variables|/Game/GameplayObjects/Interactables/BP_Key.BP_Key_C|GetKeyNum _array_element) (Variables|Default|GetMinKeyID) (Variables|Default|GetMaxKeyID))
      (Utilities|Array|Add (Variables|Default|GetKeyArray) _array_element)
      (Default|BindKeys (Variables|/Game/UI/IngameUI/WBP_IngameUI.WBP_IngameUI_C|GetWBP_Keycards (Variables|/Game/UI/WBP_GameHud.WBP_GameHud_C|GetWBP_IngameUI (Variables|/Game/PlayerControllers/BP_PlayerController.BP_PlayerController_C|GetGameHUD (Variables|/Game/Character/BP_PlayerCharacter.BP_PlayerCharacter_C|GetPlayerController (Variables|Default|Getchar))))) _array_element)))
  (Default|ShowKeys (Variables|/Game/UI/WBP_GameHud.WBP_GameHud_C|GetWBP_IngameUI (Variables|/Game/PlayerControllers/BP_PlayerController.BP_PlayerController_C|GetGameHUD (Variables|/Game/Character/BP_PlayerCharacter.BP_PlayerCharacter_C|GetPlayerController (Variables|Default|Getchar))))))

(fn DoorsInitialised
  (bind _outactors (Actor|GetAllActorsOfClass "/Game/GameplayObjects/Interactables/BP_Door_Interactable.BP_Door_Interactable_C"))
  (for _array_element _outactors
    (if (Math|Integer|InRange(Integer) (Variables|/Game/GameplayObjects/Interactables/BP_Door_Interactable.BP_Door_Interactable_C|GetDoorID _array_element) (Variables|Default|GetMinDoorID) (Variables|Default|GetMaxDoorID))
      (Default|SetManager _array_element self)
      (Utilities|Array|Add (Variables|Default|GetDoorArray) _array_element))))