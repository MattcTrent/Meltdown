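; Level streaming manager that switches the menu, hub, key maze and big room sublevels in and out, and handles quitting.
; Each area has an event that toggles load or unload through a boolean flag, with hub loading also calling OnStartGame on the game mode.
; Trigger overlaps drive hub, menu and quit.
; RespawnToMenu unloads the gameplay levels and loads the menu hidden, without updating the flags.
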(event OnActorBeginOverlap(StartGameTrig)
  (params (OverlappedActor :type Actor%20Object%20Reference) (OtherActor :type Actor%20Object%20Reference))
  (CallFunction|Load/UnloadLevel))

(event OnActorEndOverlap(QuitGameTrig)
  (params (OverlappedActor :type Actor%20Object%20Reference) (OtherActor :type Actor%20Object%20Reference))
  (CallFunction|QuitGame))

(event OnActorBeginOverlap(UnloadMenuTrig)
  (params (OverlappedActor :type Actor%20Object%20Reference) (OtherActor :type Actor%20Object%20Reference))
  (CallFunction|Load/UnloadMenu))

(event Custom|Load/Unload%20Level
  ;[1 1 1] Go Into Hub Level
  (if (Variables|Default|GetLevelHubLoaded?)
    (Game|UnloadStreamLevel(byName) "Level_Hub" false)
    (Variables|Default|SetLevelHubLoaded? false)
    (else
      (Game|LoadStreamLevel(byName) "Level_Hub" true)
      (Variables|Default|SetLevelHubLoaded? true)
      (Default|CallOnStartGame (CallFunction|GetGameMode self)))))

(event Custom|Load%20Big%20Room
  ;[1 1 1] Used To Load Big Room
  (if (Variables|Default|GetBig%20Room%20Loaded?)
    (Game|UnloadStreamLevel(byName) "Level_Big_Room" false)
    (Variables|Default|SetBig%20Room%20Loaded? false)
    (else
      (Game|LoadStreamLevel(byName) "Level_Big_Room" true)
      (Variables|Default|SetBig%20Room%20Loaded? true))))

(event Custom|Quit%20Game
  (Game|QuitGame 0 "Quit"))

(event Custom|init%20level%20stream%20manager
  (params (gm%20ref :type BP%20Persistant%20GM%20Object%20Reference))
  ;[0.1219 0 1] ADDED REFRENCE TO GM
  (Variables|Default|SetGM gm%20ref))

(event Custom|Load/Unload%20Menu
  ;[1 1 1] Used For Menu Area
  (if (Variables|Default|GetMenuLoaded?)
    (Game|UnloadStreamLevel(byName) "Level_Menu" false)
    (Variables|Default|SetMenuLoaded? false)
    (else
      (Game|LoadStreamLevel(byName) "Level_Menu" true)
      (Variables|Default|SetMenuLoaded? true))))

(event Custom|Load%20Key%20Maze
  ;[1 1 1] Used For Key Maze Room
  (if (Variables|Default|GetKeyMazeLoaded?)
    (Game|UnloadStreamLevel(byName) "Level_Key_Maze" false)
    (Variables|Default|SetKeyMazeLoaded? false)
    (else
      (Game|LoadStreamLevel(byName) "Level_Key_Maze" true)
      (Variables|Default|SetKeyMazeLoaded? true))))

(event Custom|Respawn%20To%20Menu
  (Utilities|FlowControl|Sequence
    (:then_1
      (Game|UnloadStreamLevel(byName) "Level_Hub" false))
    (:then_2
      (Game|UnloadStreamLevel(byName) "Level_Key_Maze" false))
    (:then_3
      (Game|UnloadStreamLevel(byName) "Level_Big_Room" false))
    (:then_5
      (Game|LoadStreamLevel(byName) "LeveL_Menu" false))))

(fn ConstructionScript)