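; BP_Door is an interactable door that checks whether the interacting player holds its key.
; InteractFunction calls the parent version, then indexes the KeyArray on the controller's ControlledChar with the door's DoorNum.
; It prints a debug message and returns true or false from that lookup, with no door movement in this Blueprint.
; The construction script only calls its parent.
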(fn ConstructionScript
  (|CallParentFunction))

(fn InteractFunction
  (params (Controller :type BP%20Player%20Controller%20Object%20Reference))
  (|CallParentFunction Controller)
  (if (Utilities|Array|Get(acopy) (Variables|/Game/Character/BP_PlayerCharacter.BP_PlayerCharacter_C|GetKeyArray (Variables|/Game/PlayerControllers/BP_PlayerController.BP_PlayerController_C|GetControlledChar Controller)) (Variables|Default|GetDoorNum))
    (Development|PrintString "Open the door")
    (return true)
    (else
      (Development|PrintString "Door no open, door bad")
      (return false))))