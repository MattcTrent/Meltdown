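; A key-locked double door interactable that the player opens when holding the matching key.
; Interacting while closed sets a first-door flag on the character and checks its key array, playing granted or denied audio, with a debug print when denied.
; A timeline swings both door meshes open, and the room manager records the door by ID as open.
; A reset event restores the closed rotation.
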(event Custom|ResetDoor
  (Transformation|SetRelativeRotation (Variables|Default|GetDoor1) "0,-180.000000, 0" false false)
  (Transformation|SetRelativeRotation (Variables|Default|GetDoor2) "0,180.000000, 0" false false)
  (Variables|Default|SetIsOpen false))

(event Custom|OpenDoors
  (Variables|Default|SetIsOpen true)
  (bind _openfloat (Timeline|DoorOpenTL PlayFromStart)
    (:Update
      (Transformation|SetRelativeRotation (Variables|Default|GetDoor1) (Math|Rotator|Lerp(Rotator) "0,-180.000000, 0" "0,-270.000000, 0" _openfloat) false false)
      (Transformation|SetRelativeRotation (Variables|Default|GetDoor2) (Math|Rotator|Lerp(Rotator) "0,180.000000, 0" "0,270.000000, 0" _openfloat) false false))))

(event Custom|SetManager
  (params (Manager :type BP%20Room%20Manager%20Object%20Reference))
  (Variables|Default|SetRoomManager Manager))

(fn ConstructionScript
  (|CallParentFunction))

(fn InteractFunction
  (params (Controller :type BP%20Player%20Controller%20Object%20Reference))
  (bind _controlledchar (Variables|/Game/PlayerControllers/BP_PlayerController.BP_PlayerController_C|GetControlledChar Controller))
  (|CallParentFunction Controller)
  (if (Variables|Default|GetIsOpen)
    (return false)
    (else
      (Variables|/Game/Character/BP_PlayerCharacter.BP_PlayerCharacter_C|SetFirstDoor _controlledchar true)
      (if (Utilities|Array|Get(acopy) (Variables|/Game/Character/BP_PlayerCharacter.BP_PlayerCharacter_C|GetKeyArray _controlledchar) (Variables|Default|GetKeyNum))
        (Audio|PlaySoundatLocation (Variables|Sounds|GetAccess%20Granted) (Transformation|GetActorLocation) "0, 0, 0" (Variables|Sounds|GetSound%20Vol) 1.0 0.0 "/Game/Sounds/AtLocation.AtLocation" 0 0)
        (CallFunction|OpenDoors)
        (Utilities|Array|SetArrayElem (Variables|/Game/Managers/BP_RoomManager.BP_RoomManager_C|GetOpenDoors (Variables|Default|GetRoomManager)) (Variables|Default|GetDoorID) true)
        (return true)
        (else
          (Audio|PlaySoundatLocation (Variables|Sounds|GetAccess%20Denied) (Transformation|GetActorLocation) "0, 0, 0" (Variables|Sounds|GetSound%20Vol) 1.0 0.0 "/Game/Sounds/AtLocation.AtLocation" 0 0)
          (Development|PrintString (Utilities|String|Append "I need key " (Utilities|String|ToString(Integer) (+ (Variables|Default|GetKeyNum) 1))))
          (return false))))))