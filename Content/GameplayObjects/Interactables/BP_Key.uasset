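; BP_Key is an interactable key pickup that marks its key number as held by the interacting controller's character.
; On interaction it runs the parent logic, then sets the KeyNum entry of that character's KeyArray to true.
; It then activates its particle system, hides its static mesh and disables actor collision, leaving the actor in place rather than destroying it.
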(fn ConstructionScript
  (|CallParentFunction))

(fn InteractFunction
  (params (Controller :type BP%20Player%20Controller%20Object%20Reference))
  (|CallParentFunction Controller)
  (Utilities|Array|SetArrayElem (Variables|/Game/Character/BP_PlayerCharacter.BP_PlayerCharacter_C|GetKeyArray (Variables|/Game/PlayerControllers/BP_PlayerController.BP_PlayerController_C|GetControlledChar Controller)) (Variables|Default|GetKeyNum) true)
  (Components|Activation|Activate (Variables|Default|GetParticleSystem) false)
  (Development|SetHiddeninGame (Variables|Default|GetStaticMesh) true false)
  (Collision|SetActorEnableCollision false)
  (return true))