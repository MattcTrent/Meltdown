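; Rescuable NPC interactable that picks one of three random meshes on construction and registers with the game mode and room manager.
; First interaction records the rescue by NPCID, shows dialogue, recharges the player's torch, notifies the game manager and triggers a first-save tutorial.
; A timer then plays a teleport effect, hides the NPC and disables its collision.
; AlreadySaved hides previously rescued NPCs immediately.
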(event Custom|Close%20Dialogue
  ;[1 1 1] Remove NPC once Dialogue Finished
  (Components|Activation|Activate (Variables|Default|GetTeleport) false)
  (Utilities|FlowControl|Delay 1.25)
  (Development|SetHiddeninGame (Variables|Character|GetMesh) true false)
  (Development|SetHiddeninGame (Variables|Default|GetWidget) true false)
  (Collision|SetActorEnableCollision false)
  (Components|Activation|Deactivate (Variables|Default|GetTeleport))
  (Default|CallOnHiddenfromWorld self))

(event Custom|Init
  (params (RoomManager :type BP%20Room%20Manager%20Object%20Reference))
  (bind _self self)
  ;[1 1 1] Initialise NPC
  (Default|CallOnObjectInitialised (CallFunction|GetGameMode _self) _self)
  (bind _output_get (Variables|Default|SetRoomManager RoomManager))
  (Variables|Default|SetGameManager (Variables|/Game/Managers/BP_RoomManager.BP_RoomManager_C|GetGMref _output_get)))

(event EventInteract
  (params (Controller :type BP%20Player%20Controller%20Object%20Reference))
  (bind _controlledchar (Variables|/Game/PlayerControllers/BP_PlayerController.BP_PlayerController_C|GetControlledChar Controller))
  ;[1 1 1] Interaction Function
  (if (not (Variables|Default|GetHasBeenRescued))
    (Variables|/Game/Character/BP_PlayerCharacter.BP_PlayerCharacter_C|SetFirstNPC _controlledchar true)
    (Utilities|Array|SetArrayElem (Variables|/Game/Managers/BP_RoomManager.BP_RoomManager_C|GetRescuedNPCs (Variables|Default|GetRoomManager)) (Variables|Default|GetNPC_ID) true)
    (if (Variables|/Game/Character/BP_PlayerCharacter.BP_PlayerCharacter_C|GetFirstSave _controlledchar)
      _
      (else
        (Default|SetText (.AsWBP%20Tutorial (Utilities|Casting|CastToWBP_Tutorial (UserInterface|GetUserWidgetObject (Variables|/Game/Character/BP_PlayerCharacter.BP_PlayerCharacter_C|GetWidget _controlledchar)))) "NewEnumerator6")
        (Variables|/Game/Character/BP_PlayerCharacter.BP_PlayerCharacter_C|SetFirstSave _controlledchar true)))
    (Variables|Default|SetHasBeenRescued true)
    (Development|SetHiddeninGame (Variables|Default|GetWidget) false false)
    (bind _output_get (Variables|Default|SetTorch (.AsBP%20Torch%20Actor (Utilities|Casting|CastToBP_TorchActor (Variables|/Script/Engine.ChildActorComponent|GetChildActor (Variables|/Game/Character/BP_PlayerCharacter.BP_PlayerCharacter_C|GetTorchActor _controlledchar))))))
    (Default|AddPower _output_get (Variables|Default|GetTorchRecharge))
    (Utilities|Time|SetTimerbyEvent (delegate Custom|Close%20Dialogue) 5.0)
    (Default|CallPersonSaved (Variables|Default|GetGameManager) (Variables|Default|GetRoomManager))))

(fn ConstructionScript
  (bind _mesh (Variables|Character|GetMesh))
  (Class|SkinnedMeshComponent|SetSkeletalMesh _mesh (Utilities|Select :Index (Math|Random|RandomInteger 3) :Option%200 "/Game/Art/Characters/NPCs/SM_NPC1.SM_NPC1" :Option%201 "/Game/Art/Characters/NPCs/SM_NPC2.SM_NPC2" :Option%202 "/Game/Art/Characters/NPCs/SM_NPC3.SM_NPC3") false)
  (Components|Animation|SetAnimationMode _mesh "AnimationBlueprint")
  (Components|SkeletalMesh|SetAnimInstanceClass _mesh "/Game/Art/Characters/NPCs/AB_NPCAnim.AB_NPCAnim_C"))

(fn AlreadySaved
  (Variables|Default|SetHasBeenRescued true)
  (Rendering|SetActorHiddenInGame true)
  (Collision|SetActorEnableCollision false))

(fn IconType
  (return (Variables|Default|GetIcon%20Type)))