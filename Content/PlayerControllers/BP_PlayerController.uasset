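; Player controller that spawns and possesses BP_PlayerCharacter, then sets up the game HUD and mouse cursor.
; Input drives movement along the actor's axes and sends Interact messages to overlapping actors, while Tick yaws the mesh toward the cursor hit point.
; A PlayerValid macro guards character access.
; Pause toggles the HUD's pause UI without pausing the game here, InitSM initialises the spawn manager, and Endgame is an empty stub.
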(event Custom|Spawn%20Character
  (params (Transform :type Transform))
  ;[1 1 1] Spawn Player
  (bind _returnvalue (Game|SpawnActorfromClass "/Game/Character/BP_PlayerCharacter.BP_PlayerCharacter_C" Transform "Undefined" 0 self 0))
  (bind _output_get (Variables|References|SetControlledChar _returnvalue))
  (Pawn|Possess _output_get)
  (Default|Init _output_get)
  (CallFunction|SetupUI)
  (Variables|Default|SetbShowMouseCursor true))

(event Custom|Init%20SM
  ;[1 1 1] Init Spawn Manager
  (Default|Initialise (Variables|Default|GetBP_SpawnManager) self))

(event Custom|Pause%20Game
  (bind _gamehud (Variables|Default|GetGameHUD))
  ;[1 1 1] Pause Game
  (Utilities|FlowControl|FlipFlop
    (:A
      (Default|ShowPauseUI _gamehud))
    (:B
      (Default|HidePauseUI _gamehud))))

(event Custom|Setup%20UI
  (bind _self self)
  ;[1 1 1] Setup UI
  (Utilities|IsValid (Variables|Default|GetGameHUD)
    (:Is%20Valid
      (Default|Initialise (Variables|Default|GetGameHUD)))
    (:Is%20Not%20Valid
      (bind _returnvalue (UserInterface|CreateWidget "/Game/UI/WBP_GameHud.WBP_GameHud_C" _self _self))
      (bind _output_get (Variables|Default|SetGameHUD _returnvalue))
      (UserInterface|Viewport|AddtoPlayerScreen _output_get)
      (Default|Initialise _output_get))))

(event Custom|End%20game
  ;[0.04933 0 1] called from GM use for stop player movement and other tings
)

(event EventTick
  (params (DeltaSeconds :type Float%20%28single-precision%29))
  ;[1 0.05652 0] uh oh
  (bind _controlledchar (Utilities|PlayerValid)
    (:Out
      (CallFunction|TurnPlayertoMouse _controlledchar))))

(event Input|ActionEvents|InputActionPauseGame
  (params (Key :type Key%20Structure))
  (bind _gamehud (Variables|Default|GetGameHUD))
  ;[1 1 1] Pause Game
  (:Pressed
    (Utilities|FlowControl|FlipFlop
      (:A
        (Default|ShowPauseUI _gamehud))
      (:B
        (Default|HidePauseUI _gamehud)))))

(event Input|ActionEvents|InputActionInteract
  (params (Key :type Key%20Structure))
  (:Pressed
    (bind _controlledchar (Utilities|PlayerValid)
      (:Out
        (for _array_element (Collision|GetOverlappingActors (Variables|/Game/Character/BP_PlayerCharacter.BP_PlayerCharacter_C|GetInteract%20Collision _controlledchar) 0 :!class /Script/Engine.PrimitiveComponent)
          (if (Utilities|DoesObjectImplementInterface _array_element "/Game/Interface/Interact.Interact_C")
            (Class|Interact|Interact(Message) _array_element self)
            (Development|PrintString (Utilities|GetDisplayName _array_element))))))))

(event Input|AxisEvents|InputAxisMoveForward
  (params (AxisValue :type Float%20%28single-precision%29))
  ;[1 1 1] Character Movement
  (bind _controlledchar (Utilities|PlayerValid)
    (:Out
      (Pawn|Input|AddMovementInput _controlledchar (Transformation|GetActorForwardVector _controlledchar) AxisValue false))))

(event Input|AxisEvents|InputAxisMoveRight
  (params (AxisValue :type Float%20%28single-precision%29))
  ;[1 1 1] Character Movement
  (bind _controlledchar (Utilities|PlayerValid)
    (:Out
      (Pawn|Input|AddMovementInput _controlledchar (Transformation|GetActorRightVector _controlledchar) AxisValue false))))

(fn ConstructionScript
  (|CallParentFunction))

(fn TurnPlayertoMouse
  (params (Player :type BP%20Player%20Character%20Object%20Reference))
  (Transformation|SetWorldRotation (Variables|/Script/Engine.Character|GetMesh Player) (Math|Rotator|MakeRotator 0.0 0.0 (.yaw (Math|Rotator|FindLookatRotation (Transformation|GetActorLocation Player) (.Location (Collision|BreakHitResult (.HitResult (Game|Player|GetHitResultUnderCursorbyChannel "TraceTypeQuery3" true))))))) false false))

(fn UpdateLevelName)