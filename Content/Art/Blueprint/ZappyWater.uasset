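; ZappyWater is an electrified puddle hazard that damages the player on overlap and drains their torch's power.
; A one-second timer resets a flag that throttles repeat hits, which only register on a new box overlap.
; The player's first damage also sets tutorial text on their widget.
; The construction script creates a puddle material instance from exposed colour, opacity and emissive settings, and sets the chosen cable mesh.
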(event OnComponentBeginOverlap(Box)
  (params (OverlappedComponent :type Primitive%20Component%20Object%20Reference) (OtherActor :type Actor%20Object%20Reference) (OtherComp :type Primitive%20Component%20Object%20Reference) (OtherBodyIndex :type Integer) (bFromSweep :type Boolean) (SweepResult :type Hit%20Result%20Structure%20%28by%20ref%29))
  (if (not (Variables|Default|GetRecentlyDamagedPlayer))
    (bind _asbp_player_character (Utilities|Casting|CastToBP_PlayerCharacter OtherActor))
    (Default|DamagePlayer _asbp_player_character)
    (Default|ReducePower (.AsBP%20Torch%20Actor (Utilities|Casting|CastToBP_TorchActor (Variables|/Script/Engine.ChildActorComponent|GetChildActor (Variables|/Game/Character/BP_PlayerCharacter.BP_PlayerCharacter_C|GetTorchActor _asbp_player_character)))) 5 (Transformation|GetActorLocation) true false)
    (Variables|Default|SetRecentlyDamagedPlayer true)
    (if (Variables|/Game/Character/BP_PlayerCharacter.BP_PlayerCharacter_C|GetFirstDamage _asbp_player_character)
      _
      (else
        (Default|SetText (.AsWBP%20Tutorial (Utilities|Casting|CastToWBP_Tutorial (UserInterface|GetUserWidgetObject (Variables|/Game/Character/BP_PlayerCharacter.BP_PlayerCharacter_C|GetWidget _asbp_player_character)))) "NewEnumerator7")
        (Variables|/Game/Character/BP_PlayerCharacter.BP_PlayerCharacter_C|SetFirstDamage _asbp_player_character true)))
    (Utilities|Time|SetTimerbyEvent (delegate Custom|DamageReset) 1.0)))

(event Custom|DamageReset
  (Variables|Default|SetRecentlyDamagedPlayer false))

(fn ConstructionScript
  (bind _returnvalue (Rendering|Material|CreateDynamicMaterialInstance (Variables|Default|GetPuddleMat) "Color" :!class /Script/Engine.KismetMaterialLibrary))
  (Rendering|Material|SetVectorParameterValue _returnvalue "PuddleColor" (Variables|Default|GetColour) :!class /Script/Engine.MaterialInstanceDynamic)
  (Rendering|Material|SetScalarParameterValue _returnvalue "Strength" (Variables|Default|GetOpacityStrength) :!class /Script/Engine.MaterialInstanceDynamic)
  (Rendering|Material|SetScalarParameterValue _returnvalue "EmissiveMultiplier" (Variables|Default|GetEmissiveness) :!class /Script/Engine.MaterialInstanceDynamic)
  (Components|StaticMesh|SetStaticMesh (Variables|Default|GetCableMesh) (Variables|Default|GetCableToUse)))