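; Blueprint function library of shared helpers for game framework access and UI button styling.
; Three getters return the game instance, game mode and a widget's owning player controller, cast to the project's Blueprint classes.
; SetButtonState rebuilds a button's style from a set of state images, using the hovered image as normal when the owning player's controller has user focus on it, so focused buttons appear highlighted.
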(fn GetGameInstance
  (params (WorldContextObject :type Object%20Object%20Reference))
  (bind _asbp_game_instance (Utilities|Casting|CastToBP_GameInstance (Game|GetGameInstance WorldContextObject)))
  (return _asbp_game_instance))

(fn GetGameMode
  (params (WorldContextObject :type Object%20Object%20Reference))
  (bind _asbp_persistant_gm (Utilities|Casting|CastToBP_PersistantGM (Game|GetGameMode WorldContextObject)))
  (return _asbp_persistant_gm))

(fn GetWidgetOwnerPC
  (params (Target :type Widget%20Object%20Reference))
  (bind _asbp_player_controller (Utilities|Casting|CastToBP_PlayerController (Widget|GetOwningPlayer Target)))
  (return _asbp_player_controller))

(fn SetButtonState
  (params (Button :type Button%20Object%20Reference) (States :type S%20Button%20State%20Structure))
  (bind (_normal _hovered _pressed) (Utilities|Struct|BreakS_ButtonState States))
  (bind _slatebrush (Utilities|Struct|MakeSlateBrush "(X=32.000000,Y=32.000000)" "(Left=0.000000,Top=0.000000,Right=0.000000,Bottom=0.000000)" "(SpecifiedColor=(R=1.000000,G=1.000000,B=1.000000,A=1.000000),ColorUseRule=UseColor_Specified)" _pressed "Image" "NoTile" "NoMirror"))
  (bind _slatebrush_2 (Utilities|Struct|MakeSlateBrush "(X=32.000000,Y=32.000000)" "(Left=0.000000,Top=0.000000,Right=0.000000,Bottom=0.000000)" "(SpecifiedColor=(R=1.000000,G=1.000000,B=1.000000,A=1.000000),ColorUseRule=UseColor_Specified)" _hovered "Image" "NoTile" "NoMirror"))
  (if (Class|Widget|HasUserFocus Button (CallFunction|GetWidgetOwnerPC Button Button))
    (Class|Button|SetStyle Button (Utilities|Struct|MakeButtonStyle _slatebrush_2 _slatebrush_2 _slatebrush))
    (else
      (Class|Button|SetStyle Button (Utilities|Struct|MakeButtonStyle (Utilities|Struct|MakeSlateBrush "(X=32.000000,Y=32.000000)" "(Left=0.000000,Top=0.000000,Right=0.000000,Bottom=0.000000)" "(SpecifiedColor=(R=1.000000,G=1.000000,B=1.000000,A=1.000000),ColorUseRule=UseColor_Specified)" _normal "Image" "NoTile" "NoMirror") _slatebrush_2 _slatebrush)))))