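; BP_SparksBurst is an actor that plays an intermittent spark effect by switching its particle system on and off.
; Shortly after BeginPlay, two timer-bound events begin scheduling each other in an endless loop.
; StartSpark activates the particles for a brief fixed burst, then StopSpark deactivates them and waits a random interval before the next one, giving the sparks an irregular rhythm.
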(event Custom|StartSpark
  (Components|Activation|Activate (Variables|Default|GetParticleSystem) false)
  (Utilities|Time|SetTimerbyEvent (delegate Custom|StopSpark) 0.1))

(event Custom|StopSpark
  (Components|Activation|Deactivate (Variables|Default|GetParticleSystem))
  (Utilities|Time|SetTimerbyEvent (delegate Custom|StartSpark) (Math|Random|RandomFloatinRange 0.3 0.6)))

(event EventBeginPlay
  (Utilities|Time|SetTimerbyEvent (delegate Custom|StartSpark) 0.1))

(fn ConstructionScript)