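; Steam nozzle hazard that periodically vents gas and drains the player's torch power on contact.
; A looping timer toggles the Gas particle emitter and its EmitterOn flag on and off.
; While on, box begin-overlap events reduce the player's child torch actor power, with a short timer-reset cooldown between hits.
; The player's first hit also sets tutorial widget text, guarded by a flag on the player character.
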(event OnComponentBeginOverlap(Box)
  (params (OverlappedComponent :type Primitive%20Component%20Object%20Reference) (OtherActor :type Actor%20Object%20Reference) (OtherComp :type Primitive%20Component%20Object%20Reference) (OtherBodyIndex :type Integer) (bFromSweep :type Boolean) (SweepResult :type Hit%20Result%20Structure%20%28by%20ref%29))
  (if (Variables|Default|GetEmitterOn)
    (if (not (Variables|Default|GetRecentlyDamagedPlayer))
      (bind _asbp_player_character (Utilities|Casting|CastToBP_PlayerCharacter OtherActor))
      (Default|ReducePower (.AsBP%20Torch%20Actor (Utilities|Casting|CastToBP_TorchActor (Variables|/Script/Engine.ChildActorComponent|GetChildActor (Variables|/Game/Character/BP_PlayerCharacter.BP_PlayerCharacter_C|GetTorchActor _asbp_player_character)))) 5)
      (Variables|Default|SetRecentlyDamagedPlayer true)
      (if (Variables|/Game/Character/BP_PlayerCharacter.BP_PlayerCharacter_C|GetFirstDamage _asbp_player_character)
        _
        (else
          (Default|SetText (.AsWBP%20Tutorial (Utilities|Casting|CastToWBP_Tutorial (UserInterface|GetUserWidgetObject (Variables|/Game/Character/BP_PlayerCharacter.BP_PlayerCharacter_C|GetWidget _asbp_player_character)))) "NewEnumerator7")
          (Variables|/Game/Character/BP_PlayerCharacter.BP_PlayerCharacter_C|SetFirstDamage _asbp_player_character true)))
      (Utilities|Time|SetTimerbyEvent (delegate Custom|DamageReset) 1.0))))

(event Custom|DamageReset
  (Variables|Default|SetRecentlyDamagedPlayer false))

(event Custom|StopGas
  (Effects|Components|ParticleSystem|SetEmitterEnable (Variables|Default|GetParticleSystem) "Gas" false)
  (Variables|Default|SetEmitterOn false))

(event Custom|StartGas
  (Effects|Components|ParticleSystem|SetEmitterEnable (Variables|Default|GetParticleSystem) "Gas" true)
  (Variables|Default|SetEmitterOn true))

(event Custom|ChangeState
  (if (Variables|Default|GetEmitterOn)
    (CallFunction|StopGas)
    (else
      (CallFunction|StartGas))))

(event EventBeginPlay
  (Utilities|Time|SetTimerbyEvent (delegate Custom|ChangeState) 5.0 true))

(fn ConstructionScript)